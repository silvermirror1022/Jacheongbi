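; BP_spriteCharacter is a 2D Paper2D player character that runs left and right and jumps.
; Axis input moves it along world X, and the Jump action triggers a jump.
; Each Tick switches the flipbook between run and idle by velocity, then sets controller yaw to 0 or 180 from the sign of X velocity to face the movement direction.
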(event `self.ReceiveTick`
  (params (DeltaSeconds :type "Float (single-precision)"))
  (`self.애니메이션`)
  (`self.회전 제어`))

(event `InputAxis|move Right`
  (params (AxisValue :type "Float (single-precision)"))
  (`self.AddMovementInput` (1.0 0.0 0.0) AxisValue))

(event `InputAction|Jump`
  (params (Key :type "Key Structure"))
  (:`Pressed`
    (`self.Jump`)))

(event `애니메이션`
  (`PaperFlipbookComponent.SetFlipbook` (`self.Sprite`) (select `bool` (> (`KismetMathLibrary.VSize` (`MovementComponent.Velocity` (`self.CharacterMovement`))) 0.0) :`false` "/Game/PNG/sprites/player/idle/player-idle.player-idle" :`true` "/Game/PNG/sprites/player/run/player-run.player-run" :!type "PaperFlipbook Object Reference")))

(event `회전 제어`
  (`/Engine/EditorBlueprintResources/StandardMacros.IsValid` (`self.GetController`)
    (:`Is Valid`
      (`/Engine/EditorBlueprintResources/StandardMacros.CompareFloat` (.x (`MovementComponent.Velocity` (`self.CharacterMovement`)))
        (:`>`
          (`Controller.SetControlRotation` (`self.GetController`) (`KismetMathLibrary.MakeRotator` 0.0)))
        (:`<`
          (`Controller.SetControlRotation` (`self.GetController`) (`KismetMathLibrary.MakeRotator` 0.0 0.0 180.0)))))))

(fn `UserConstructionScript`)